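; BP_CutSceneManager starts the image-based cutscene that matches the current cutscene level.
; On BeginPlay it creates WBP_PlayCutScene, adds it to the viewport and switches on the level name to pick that scene's image set.
; It hands the widget those images and the next level's name, either Level_1 or MainMenu, then calls AddImageToDisplay to begin showing them.
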(event EventBeginPlay
  (bind _returnvalue (UserInterface|CreateWidget "/Game/Blueprints/Widgets/WBP_PlayCutScene.WBP_PlayCutScene_C"))
  (UserInterface|Viewport|AddtoViewport _returnvalue 0)
  (bind _returnvalue_2 (Game|GetCurrentLevelName true))
  (switch string _returnvalue_2
    (:CutScene1
      (Default|GetSceneImages _returnvalue (Variables|Default|GetCutSceneImagesScene1))
      (Default|GetNextLevelName _returnvalue "Level_1"))
    (:CutScene2
      (Default|GetSceneImages _returnvalue (Variables|Default|GetCutSceneImagesScene2))
      (Default|GetNextLevelName _returnvalue "MainMenu")))
  (Default|AddImagetoDisplay _returnvalue))

(event EventTick
  (params (DeltaSeconds :type Float%20%28single-precision%29)))

(fn ConstructionScript)