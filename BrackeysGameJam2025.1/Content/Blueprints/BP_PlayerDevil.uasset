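; Player devil Blueprint that handles the invisibility visual effect and opens the pause and game-over menus.
; Turning invisible creates dynamic material instances for the face and body mesh and lowers their opacity parameters, which BecomeVisible restores on those stored instances.
; Separate events add the pause widget, or the reset-level widget after a short delay, and IsPlayer reports whether it is player-controlled.
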(event EventBeginPlay)

(event Collision|EventActorBeginOverlap
  (params (OtherActor :type Actor%20Object%20Reference)))

(event EventTick
  (params (DeltaSeconds :type Float%20%28single-precision%29)))

(event EventApplyTurnInvisibleEffect
  (bind _mesh (Variables|Character|GetMesh))
  (bind _devilface (Variables|Default|GetDevilFace))
  (Utilities|FlowControl|Sequence
    (:then_0
      (bind _returnvalue (Rendering|Material|CreateDynamicMaterialInstance _devilface 0 (Rendering|Material|GetMaterial _devilface 0) "None" :!class /Script/Engine.PrimitiveComponent))
      (Variables|Default|SetDevilFaceMaterial _returnvalue)
      (Rendering|Material|SetMaterial (Variables|Default|GetDevilFace) 0 (Variables|Default|GetDevilFaceMaterial))
      (Rendering|Material|SetScalarParameterValue (Variables|Default|GetDevilFaceMaterial) "TransluscentParm" 0.7 :!class /Script/Engine.MaterialInstanceDynamic))
    (:then_1
      (bind _returnvalue_2 (Rendering|Material|CreateDynamicMaterialInstance _mesh 0 (Rendering|Material|GetMaterial _mesh 0) "None" :!class /Script/Engine.PrimitiveComponent))
      (Variables|Default|SetMeshMaterial _returnvalue_2)
      (Rendering|Material|SetMaterial (Variables|Character|GetMesh) 0 (Variables|Default|GetMeshMaterial))
      (Rendering|Material|SetScalarParameterValue (Variables|Default|GetMeshMaterial) "Opacity" 0.4 :!class /Script/Engine.MaterialInstanceDynamic))))

(event EventBecomeVisible
  (Utilities|FlowControl|Sequence
    (:then_0
      (Rendering|Material|SetScalarParameterValue (Variables|Default|GetDevilFaceMaterial) "TransluscentParm" 1.0 :!class /Script/Engine.MaterialInstanceDynamic))
    (:then_1
      (Rendering|Material|SetScalarParameterValue (Variables|Default|GetMeshMaterial) "Opacity" 1.0 :!class /Script/Engine.MaterialInstanceDynamic))))

(event EventPauseGame
  (params (Value :type Input%20Action%20Value%20Structure%20%28by%20ref%29))
  (bind _returnvalue (UserInterface|CreateWidget "/Game/Blueprints/Widgets/WBP_PauseMenu.WBP_PauseMenu_C"))
  (UserInterface|Viewport|AddtoViewport _returnvalue 0))

(event EventShowGameOverWidget
  (Utilities|FlowControl|Delay 0.2)
  (bind _returnvalue (UserInterface|CreateWidget "/Game/Blueprints/Widgets/WBP_ResetLevel.WBP_ResetLevel_C"))
  (UserInterface|Viewport|AddtoViewport _returnvalue 0))

(fn ConstructionScript)

(fn IsPlayer
  (return (Pawn|IsPlayerControlled)))