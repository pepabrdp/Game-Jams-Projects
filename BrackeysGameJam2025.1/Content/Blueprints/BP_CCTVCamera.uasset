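; Security camera that sweeps for the player devil, then locks on and shoots once it detects them.
; While searching, it interpolates between lower, middle and upper rotators using an orientation state.
; Vision cone overlap and Tick checks set detection unless the player is invisible, recoloring the cone through a dynamic material.
; A looping BeginPlay timer spawns projectiles only while detected; invisibility or leaving the cone resets detection.
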(event OnComponentBeginOverlap(VisionCone)
  (params (OverlappedComponent :type Primitive%20Component%20Object%20Reference) (OtherActor :type Actor%20Object%20Reference) (OtherComp :type Primitive%20Component%20Object%20Reference) (OtherBodyIndex :type Integer) (bFromSweep :type Boolean) (SweepResult :type Hit%20Result%20Structure%20%28by%20ref%29))
  (bind _isplayer (Class|BPIPlayer|IsPlayer(Message) OtherActor))
  (if _isplayer
    (CallFunction|CheckifPlayerIsDetactable (Variables|Default|GetPlayer%20Devil))))

(event OnComponentEndOverlap(VisionCone)
  (params (OverlappedComponent :type Primitive%20Component%20Object%20Reference) (OtherActor :type Actor%20Object%20Reference) (OtherComp :type Primitive%20Component%20Object%20Reference) (OtherBodyIndex :type Integer))
  (bind _isplayer (Class|BPIPlayer|IsPlayer(Message) OtherActor))
  (if (and _isplayer (Variables|Default|GetPlayerDetected))
    (CallFunction|ResetPlayerDetected)))

(event EventBeginPlay
  (Variables|Default|SetInitialCameraBaseRotation (Variables|/Script/Engine.SceneComponent|GetRelativeRotation (Variables|Default|GetCameraBase)))
  (bind _asbp_player_devil (Utilities|Casting|CastToBP_PlayerDevil (Pawn|GetControlledPawn (Game|GetPlayerController 0))))
  (Variables|Default|SetPlayer%20Devil _asbp_player_devil)
  (bind _returnvalue (Utilities|Time|SetTimerbyFunctionName 0 "Shoot" 1.0 true))
  (Variables|Default|SetShootTimerHandle _returnvalue))

(event Collision|EventActorBeginOverlap
  (params (OtherActor :type Actor%20Object%20Reference)))

(event EventTick
  (params (DeltaSeconds :type Float%20%28single-precision%29))
  (if (> (Utilities|Array|Length (Collision|GetOverlappingActors "/Game/Blueprints/BP_PlayerDevil.BP_PlayerDevil_C" :!class /Script/Engine.Actor)) 0)
    (if (Variables|Default|GetPlayerDetected)
      (bind _returnvalue (CallFunction|IsPlayerInvisible (Variables|Default|GetPlayer%20Devil)))
      (if _returnvalue
        (CallFunction|ResetPlayerDetected)
        (else
          (CallFunction|LockandShoot DeltaSeconds (Variables|Default|GetPlayer%20Devil))))
      (else
        (CallFunction|CheckifPlayerIsDetactable (Variables|Default|GetPlayer%20Devil))
        (CallFunction|RotatetoFindPlayer DeltaSeconds)))
    (else
      (CallFunction|RotatetoFindPlayer DeltaSeconds))))

(fn ConstructionScript)

(fn RotatetoFindPlayer
  (params (DeltaSec :type Float%20%28double-precision%29))
  (switch int (Variables|Default|GetOrientation)
    (:-1
      (CallFunction|RotatetoTargetRotator (Variables|Default|GetLowerBoundRotator) DeltaSec))
    (:0
      (if (== (Variables|Default|GetPrevOrientation) 1)
        (CallFunction|RotatetoTargetRotator (Variables|Default|GetMiddleWayRotator) DeltaSec -1)
        (else
          (CallFunction|RotatetoTargetRotator (Variables|Default|GetMiddleWayRotator) DeltaSec 1))))
    (:1
      (CallFunction|RotatetoTargetRotator (Variables|Default|GetUpperBoundRotator) DeltaSec))))

(fn LockandShoot
  (params (DeltaSec :type Float%20%28double-precision%29) (PlayerDevil :type BP%20Player%20Devil%20Object%20Reference))
  (bind _camerabase (Variables|Default|GetCameraBase))
  (Utilities|FlowControl|Sequence
    (:then_0
      ;[1 1 1] Rotate/Focus on player
      (Transformation|SetWorldRotation _camerabase (Math|Rotator|FindLookatRotation (Transformation|GetWorldLocation _camerabase) (Transformation|GetActorLocation PlayerDevil)) false false))))

(fn CheckifPlayerIsDetactable
  (params (PlayerDevil :type Player%20Devil%20Object%20Reference))
  (bind _visioncone (Variables|Default|GetVisionCone))
  (bind _returnvalue (CallFunction|IsPlayerInvisible PlayerDevil))
  (if (not _returnvalue)
    (bind _returnvalue_2 (Rendering|Material|CreateDynamicMaterialInstance _visioncone 0 (Rendering|Material|GetMaterial _visioncone 0) "None" :!class /Script/Engine.PrimitiveComponent))
    (Variables|Default|SetDynamicMaterial _returnvalue_2)
    (Rendering|Material|SetMaterial (Variables|Default|GetVisionCone) 0 (Variables|Default|GetDynamicMaterial))
    (Rendering|Material|SetVectorParameterValue (Variables|Default|GetDynamicMaterial) "Base Color" "(R=0.392157,G=0.003922,B=0.000000,A=1.000000)" :!class /Script/Engine.MaterialInstanceDynamic)
    (Variables|Default|SetPlayerDetected true)))

(fn IsPlayerInvisible
  (params (PlayerDevil :type Player%20Devil%20Object%20Reference))
  (return (Class|PlayerDevil|IsPlayerInvisible PlayerDevil)))

(fn ResetPlayerDetected
  (bind _dynamicmaterial (Variables|Default|GetDynamicMaterial))
  (Rendering|Material|SetMaterial (Variables|Default|GetVisionCone) 0 _dynamicmaterial)
  (Rendering|Material|SetVectorParameterValue _dynamicmaterial "Base Color" "(R=0.039216,G=0.345098,B=0.000000,A=1.000000)" :!class /Script/Engine.MaterialInstanceDynamic)
  (Variables|Default|SetPlayerDetected false))

(fn RotatetoTargetRotator
  (params (TargetRotator :type Rotator) (DeltaTime :type Float%20%28single-precision%29) (NewOrientation :type Integer))
  (Transformation|SetRelativeRotation (Variables|Default|GetCameraBase) (Math|Interpolation|RInterpTo (Variables|/Script/Engine.SceneComponent|GetRelativeRotation (Variables|Default|GetCameraBase)) TargetRotator DeltaTime 0.5) false false)
  (if (Utilities|Operators|EqualEqual (Variables|/Script/Engine.SceneComponent|GetRelativeRotation (Variables|Default|GetCameraBase)) TargetRotator 2.0)
    (Variables|Default|SetPrevOrientation (Variables|Default|GetOrientation))
    (Variables|Default|SetOrientation NewOrientation)))

(fn Shoot
  (if (Variables|Default|GetPlayerDetected)
    (Class|TraceUtilLibrary|TraceBookmark "CCTV Camera SHOOTS")
    (bind _returnvalue (Game|SpawnActorfromClass "/Game/Blueprints/BP_Projectile.BP_Projectile_C" (Math|Transform|MakeTransform (Transformation|GetWorldLocation (Variables|Default|GetSpawnProjectilePoint)) (Transformation|GetWorldRotation (Variables|Default|GetCameraBase)) "1.000000,1.000000,1.000000") "AdjustIfPossibleButAlwaysSpawn" "MultiplyWithRoot" 0 0))
    (Collision|IgnoreActorwhenMoving (Variables|/Script/DevilsMayhem.Projectile|GetProjectile _returnvalue) self true)
    (Collision|IgnoreActorwhenMoving (Variables|Default|GetVisionCone) _returnvalue true)
    (Actor|SetOwner _returnvalue self)
    (Variables|Default|SetShooting false)))