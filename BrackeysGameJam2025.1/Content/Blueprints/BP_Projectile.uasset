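; BP_Projectile is a projectile that launches toward the player's BP_PlayerDevil pawn when it spawns.
; On BeginPlay it casts and stores that pawn, then multiplies the offset to it by the movement component's InitialSpeed.
; The unnormalized result is set as local-space velocity, so speed scales with distance and spawn rotation affects direction.
; Aim is set only once; the file has no homing or overlap logic.
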(event EventBeginPlay
  (bind _projectilemovecomp (Variables|Default|GetProjectileMoveComp))
  (bind _asbp_player_devil (Utilities|Casting|CastToBP_PlayerDevil (Pawn|GetControlledPawn (Game|GetPlayerController 0))))
  (bind _output_get (Variables|Default|SetAs%20BP%20Player%20Devil _asbp_player_devil))
  (Game|Components|ProjectileMovement|SetVelocityinLocalSpace _projectilemovecomp (* (Variables|/Script/Engine.ProjectileMovementComponent|GetInitialSpeed _projectilemovecomp) (- (Transformation|GetActorLocation _output_get) (Transformation|GetActorLocation)))))

(event Collision|EventActorBeginOverlap
  (params (OtherActor :type Actor%20Object%20Reference)))

(event EventTick
  (params (DeltaSeconds :type Float%20%28single-precision%29)))

(fn ConstructionScript)